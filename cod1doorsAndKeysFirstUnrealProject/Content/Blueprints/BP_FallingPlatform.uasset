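; Falling platform that drops after the third-person character enters its box trigger, then returns to where it started.
; A ready flag gates activation, which waits a short delay, plays a click sound and enables physics simulation on the platform.
; After the fall duration, physics switches off and a timeline lerps the transform back to the one saved at BeginPlay, then re-arms it.
; Material swaps mark each state, alongside debug prints.
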(event OnComponentBeginOverlap(BoxTrigger)
  (params (OverlappedComponent :type Primitive%20Component%20Object%20Reference) (OtherActor :type Actor%20Object%20Reference) (OtherComp :type Primitive%20Component%20Object%20Reference) (OtherBodyIndex :type Integer) (bFromSweep :type Boolean) (SweepResult :type Hit%20Result%20Structure%20%28by%20ref%29))
  (Development|PrintString "Something is standing on me") ; string for testing alert purposes, remove later
  (Utilities|Casting|CastToBP_ThirdPersonCharacter OtherActor) ; Determines what actor activates the trigger\nin this case, the player
  (if (Variables|Default|GetisReady)
    (CallFunction|Activate)
    (else
      (Development|PrintString "Platform not ready"))))

(event Custom|Activate
  (Variables|Default|SetisReady false)
  (Rendering|Material|SetMaterial (Variables|Default|GetPlatform) 0 "/Game/Materials/FallingMaterials/MI_ActivePlatform.MI_ActivePlatform")
  (Development|PrintString "Starting coutndown")
  (Utilities|FlowControl|Delay (Variables|PlatformSettings|GetFallDelayDuration)) ; wait half a second
  (Audio|PlaySoundatLocation "/Game/SoundFX/old-radio-button-click-97549.old-radio-button-click-97549" (Transformation|GetWorldScale (Variables|Default|GetPlatform)) "0, 0, 0" 1.0 1.0 0.0 0 0 0 0)
  (CallFunction|Falling))

(event Custom|Falling
  (Rendering|Material|SetMaterial (Variables|Default|GetPlatform) 0 "/Game/Materials/FallingMaterials/MI_FallingPlatform.MI_FallingPlatform")
  (Development|PrintString "Falling")
  (Physics|SetSimulatePhysics (Variables|Default|GetPlatform) true) ; Allows platform to be affected by physics\n(gravity)
  (Utilities|FlowControl|Delay (Variables|PlatformSettings|GetFallDuration))
  (CallFunction|ResetPlatform))

(event Custom|ResetPlatform
  (Rendering|Material|SetMaterial (Variables|Default|GetPlatform) 0 "/Game/Materials/FallingMaterials/MI_ResettingPlatform.MI_ResettingPlatform")
  (Development|PrintString "Reset platform")
  (Physics|SetSimulatePhysics (Variables|Default|GetPlatform) false)
  (Variables|Default|SetFallenTransform (Transformation|GetWorldTransform (Variables|Default|GetPlatform))) ; get and set location of platform\nbefore we start resetting it
  (Rendering|Material|SetMaterial (Variables|Default|GetPlatform) 0 "/Game/Materials/FallingMaterials/MI_ResettingPlatform.MI_ResettingPlatform")
  (bind _newtrack_0 (Timeline|Return%20to%20PlatformStartTrans PlayFromStart)
    (:Update
      (Transformation|SetWorldTransform (Variables|Default|GetPlatform) (Math|Transform|Lerp(Transform) (Variables|Default|GetFallenTransform) (Variables|Default|GetPlatformStartTrans) _newtrack_0) false false))
    (:Finished
      (Variables|Default|SetisReady true)
      (Rendering|Material|SetMaterial (Variables|Default|GetPlatform) 0 "/Game/Materials/FallingMaterials/MI_ReadyPlatform.MI_ReadyPlatform"))))

(event EventBeginPlay
  (Variables|Default|SetPlatformStartTrans (Transformation|GetWorldTransform (Variables|Default|GetPlatform)))
  (Variables|Default|SetisReady true))

(fn ConstructionScript)